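; BP_PNJ is an interactable NPC that switches between a dialogue-style view with visible text and normal top-down play.
; Pressing E or calling Interact drives a FlipFlop.
; The first state shows TextRender1, blends the camera to the NPC, blocks movement through the controller's CanMove flag and hides the player pawn.
; The next call reverses all of it, blending the view back to the pawn.
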(event EventInteract
  (bind _player_controller (CallFunction|GetTopDownController))
  (bind _player_controller_2 (CallFunction|GetTopDownController))
  (bind _returnvalue (Pawn|GetControlledPawn _player_controller))
  (Utilities|FlowControl|FlipFlop
    (:A
      (Rendering|SetVisibility (Variables|Default|GetTextRender1) true false)
      (Game|Player|SetViewTargetwithBlend _player_controller_2 self 0.5 "VTBlend_Linear" 0.0 false)
      (Variables|/Game/TopDown/Blueprints/BP_TopDownController.BP_TopDownController_C|SetCanMove _player_controller_2 false)
      (Rendering|SetActorHiddenInGame (Pawn|GetControlledPawn _player_controller_2) true))
    (:B
      (Rendering|SetVisibility (Variables|Default|GetTextRender1) false false)
      (Game|Player|SetViewTargetwithBlend _player_controller _returnvalue 0.5 "VTBlend_Linear" 0.0 false)
      (Variables|/Game/TopDown/Blueprints/BP_TopDownController.BP_TopDownController_C|SetCanMove _player_controller true)
      (Rendering|SetActorHiddenInGame _returnvalue false))))

(event Input|KeyboardEvents|E
  (params (Key :type Key%20Structure))
  (:Pressed
    (CallFunction|Interact)))

(fn ConstructionScript
  (|CallParentFunction))