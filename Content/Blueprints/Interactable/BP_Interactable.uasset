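; Base interactable actor for a top-down game, with an empty Interact event and a text prompt.
; Its sphere overlap registers or removes it with the top-down controller when BP_TopDownCharacter enters or leaves.
; Each Tick shows the text only while this actor is the controller's current interactable, and rotates visible text to face the camera.
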(event OnComponentBeginOverlap(Sphere)
  (params (OverlappedComponent :type Primitive%20Component%20Object%20Reference) (OtherActor :type Actor%20Object%20Reference) (OtherComp :type Primitive%20Component%20Object%20Reference) (OtherBodyIndex :type Integer) (bFromSweep :type Boolean) (SweepResult :type Hit%20Result%20Structure%20%28by%20ref%29))
  (Utilities|Casting|CastToBP_TopDownCharacter OtherActor)
  (Default|SetInteractable (CallFunction|GetTopDownController) self))

(event OnComponentEndOverlap(Sphere)
  (params (OverlappedComponent :type Primitive%20Component%20Object%20Reference) (OtherActor :type Actor%20Object%20Reference) (OtherComp :type Primitive%20Component%20Object%20Reference) (OtherBodyIndex :type Integer))
  (Utilities|Casting|CastToBP_TopDownCharacter OtherActor)
  (Default|RemoveInteractable (CallFunction|GetTopDownController) self)
  (Rendering|SetVisibility (Variables|Default|GetTextRender) false false))

(event Custom|Interact)

(event EventTick
  (params (DeltaSeconds :type Float%20%28single-precision%29))
  (bind _textrender (Variables|Default|GetTextRender))
  (Utilities|FlowControl|Sequence
    (:then_0
      (bind (_isvalid _current_interactable) (Default|GetCurrentInteractable (CallFunction|GetTopDownController)))
      (if _isvalid
        (Rendering|SetVisibility (Variables|Default|GetTextRender) (== self _current_interactable) false)))
    (:then_1
      (if (Rendering|IsVisible _textrender)
        (Transformation|SetWorldRotation (Variables|Default|GetTextRender) (Math|Rotator|FindLookatRotation (Transformation|GetWorldLocation _textrender) (Camera|GetCameraLocation (Variables|/Script/Engine.PlayerController|GetPlayerCameraManager (CallFunction|GetTopDownController)))) false false)))))

(fn ConstructionScript)