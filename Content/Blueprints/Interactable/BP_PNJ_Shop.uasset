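; BP_PNJ_Shop is an interactable shop NPC that opens a shop interface when the player interacts with it.
; Interact blends the view to the NPC, shows its widget, initializes WBP_Shop with itself and disables movement through GetTopDownChara.
; ExitSop hides the widget, re-enables movement and calls a view blend with no target specified, then prints a debug message.
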(event Custom|ExitSop
  (Rendering|SetVisibility (Variables|Default|GetWidget) false false)
  (Variables|/Game/TopDown/Blueprints/BP_TopDownController.BP_TopDownController_C|SetCanMove (CallFunction|GetTopDownChara) true)
  (Game|Player|SetViewTargetwithBlend (CallFunction|GetTopDownChara) 0 1.0 "VTBlend_Linear" 0.0 false)
  (Development|PrintString "Out"))

(event EventInteract
  (bind _widget (Variables|Default|GetWidget))
  (Game|Player|SetViewTargetwithBlend (CallFunction|GetTopDownChara) self 1.0 "VTBlend_Linear" 1.0 false)
  (Rendering|SetVisibility _widget true false)
  (bind _aswbp_shop (Utilities|Casting|CastToWBP_Shop (UserInterface|GetWidget _widget)))
  (Default|InitializeShop _aswbp_shop self)
  (Variables|/Game/TopDown/Blueprints/BP_TopDownController.BP_TopDownController_C|SetCanMove (CallFunction|GetTopDownChara) false))

(fn ConstructionScript
  (|CallParentFunction))