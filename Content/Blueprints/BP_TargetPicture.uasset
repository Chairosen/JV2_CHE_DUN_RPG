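; BP_TargetPicture is a display actor that mirrors the look of the character referenced by Chara, apparently for a target picture.
; On BeginPlay it takes Chara's first skeletal mesh component and copies that component's mesh asset and animation class onto its own SkeletalMesh.
; The copy happens once, and the construction script only calls the parent.
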(event EventBeginPlay
  (bind _chara (Variables|Default|GetChara))
  (bind _returnvalue (Actor|GetComponentsbyTag _chara "/Script/Engine.SkeletalMeshComponent" "None"))
  (bind _output (Utilities|Array|Get(acopy) _returnvalue))
  (Components|SkeletalMesh|SetSkeletalMeshAsset (Variables|Default|GetSkeletalMesh) (Components|SkeletalMesh|GetSkeletalMeshAsset _output))
  (Components|SkeletalMesh|SetAnimInstanceClass (Variables|Default|GetSkeletalMesh) (Variables|/Script/Engine.SkeletalMeshComponent|GetAnimClass _output)))

(fn ConstructionScript
  (|CallParentFunction))