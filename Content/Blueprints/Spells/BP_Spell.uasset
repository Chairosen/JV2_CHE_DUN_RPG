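; BP_Spell is a spell projectile launched horizontally toward the player's current target.
; On BeginPlay, it sets its Sphere to probe-only collision and applies a velocity-change impulse along the player-to-target vector from the top-down controller's Targeted actor.
; The vector has Z zeroed but is not normalized, so launch speed scales with distance.
; The Sphere1 overlap event is empty, so no hit logic runs here.
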(event OnComponentBeginOverlap(Sphere1)
  (params (OverlappedComponent :type Primitive%20Component%20Object%20Reference) (OtherActor :type Actor%20Object%20Reference) (OtherComp :type Primitive%20Component%20Object%20Reference) (OtherBodyIndex :type Integer) (bFromSweep :type Boolean) (SweepResult :type Hit%20Result%20Structure%20%28by%20ref%29)))

(event EventTick
  (params (DeltaSeconds :type Float%20%28single-precision%29)))

(event EventBeginPlay
  (bind _returnvalue (Game|GetPlayerCharacter 0))
  (bind _player_controller (CallFunction|GetTopDownController))
  (bind _sphere (Variables|Default|GetSphere))
  (bind _returnvalue_2 (Transformation|GetActorLocation _returnvalue))
  (bind _targeted (Variables|/Game/TopDown/Blueprints/BP_TopDownController.BP_TopDownController_C|GetTargeted _player_controller))
  (bind _returnvalue_3 (Transformation|GetActorLocation _targeted))
  (Collision|SetCollisionEnabled _sphere "ProbeOnly")
  (Physics|AddImpulse _sphere (* (Math|Vector|MakeVector (- (.x _returnvalue_3) (.x _returnvalue_2)) (- (.y _returnvalue_3) (.y _returnvalue_2)) (- (.z _returnvalue_3) (.z _returnvalue_2))) "1.000000,1.000000,0.000000") "None" true))

(fn ConstructionScript)