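; BP_GoblinPawn is a goblin pawn that the player can target with the mouse and damage until it dies.
; Cursor hover on its Sphere registers or clears it as the top-down controller's Targetable and switches the mouse cursor.
; LooseHP subtracts damage from health set at BeginPlay, pushes the health ratio to the controller's health UI, and calls Death to destroy the actor at zero.
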(event OnBeginCursorOver(Sphere)
  (params (TouchedComponent :type Primitive%20Component%20Object%20Reference))
  (bind _player_controller (CallFunction|GetTopDownController))
  (Variables|/Game/TopDown/Blueprints/BP_TopDownController.BP_TopDownController_C|SetTargetable _player_controller self)
  (Variables|/Script/Engine.PlayerController|SetCurrentMouseCursor _player_controller "Custom"))

(event OnEndCursorOver(Sphere)
  (params (TouchedComponent :type Primitive%20Component%20Object%20Reference))
  (bind _player_controller (CallFunction|GetTopDownController))
  (Variables|/Game/TopDown/Blueprints/BP_TopDownController.BP_TopDownController_C|SetTargetable _player_controller 0)
  (Variables|/Script/Engine.PlayerController|SetCurrentMouseCursor _player_controller "Default"))

(event Custom|LooseHP
  (params (damages :type Float%20%28double-precision%29))
  (bind _output_get (Variables|Default|SetHP (- (Variables|Default|GetHP) damages)))
  (Default|SetTargetHelthPercent (Variables|/Game/TopDown/Blueprints/BP_TopDownController.BP_TopDownController_C|GetUIHealth (CallFunction|GetTopDownController)) (/ (Variables|Default|GetHP) (Variables|Default|GetHPMax)))
  (if (<= _output_get 0.0)
    (CallFunction|Death)))

(event Custom|Death
  (Actor|DestroyActor))

(event EventBeginPlay
  (bind _output_get (Variables|Default|SetHPMax 5e+01))
  (Variables|Default|SetHP _output_get))

(fn ConstructionScript)